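; BP_Stand is a shooting-gallery stand that pops up five duck targets at random.
; A loop gated on CurrentScore waits a short random delay, picks a target, and rotates it up with a timeline.
; Finished flips pass the target through an interface message into a queue.
; After a delay, a second timeline lays the front target back down and removes it from the queue.
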(event `self.ReceiveBeginPlay`
  (bind _targettedduck (`self.targettedDuck`))
  (bind _selection (`self.Selection`))
  ; Checks if the player has enough points (will be stored in a variable contained in the player
  (set `self.CurrentScore` 0.0)
  (if (not (>= (`self.CurrentScore`) 1000.0)) :!label _label
    ; Random  value for delay between a new sign popping up
    (`KismetSystemLibrary.Delay` (`KismetMathLibrary.RandomFloatInRange` 0.3 0.8))
    ; Select which target will be flipped based on the selection
    (switch `/Game/BARTOSZ_BLUEPRINTS/Enum_StandUp` (`|GetArrayItem` _selection (`KismetMathLibrary.RandomIntegerInRange` 0 (`KismetArrayLibrary.Array_LastIndex` _selection)))
      (:`NewEnumerator0`
        (set `self.targettedDuck` (`self.shoot1`))
        (bind (_direction _ducky) (`Timeline|DuckRotation` :!via `PlayFromStart` :!label _label_2)
          (:`Update`
            ; flicks the assigned target up
            (`SceneComponent.K2_SetRelativeRotation` _targettedduck (`KismetMathLibrary.RLerp` (`SceneComponent.RelativeRotation` _targettedduck) (struct) _ducky) false false)
            ; signals that a new target can be turned up
            (`/Engine/EditorBlueprintResources/StandardMacros.DoOnce` false :!label _label_3
              (:`Completed`
                (goto _label))))
          (:`Finished`
            ; async function call
            (message `/Game/BARTOSZ_BLUEPRINTS/BPI_TargetLinger.NewFunction` self (`self.targettedDuck`))
            (goto _label_3 :!via `Reset`))))
      (:`NewEnumerator1`
        (set `self.targettedDuck` (`self.shoot2`))
        (goto _label_2 :!via `PlayFromStart`))
      (:`NewEnumerator2`
        (set `self.targettedDuck` (`self.shoot3`))
        (goto _label_2 :!via `PlayFromStart`))
      (:`NewEnumerator3`
        (set `self.targettedDuck` (`self.shoot4`))
        (goto _label_2 :!via `PlayFromStart`))
      (:`NewEnumerator4`
        (set `self.targettedDuck` (`self.shoot5`))
        (goto _label_2 :!via `PlayFromStart`)))))

(event `/Game/BARTOSZ_BLUEPRINTS/BPI_TargetLinger.NewFunction`
  (params (NewParam :type "StaticMeshComponent Object Reference"))
  (bind _queue (`self.Queue`))
  (bind _output (`|GetArrayItem` (`self.Queue`)))
  ; adds the flipped target to a queue
  (`KismetArrayLibrary.Array_Add` (`self.Queue`) NewParam)
  (`KismetSystemLibrary.Delay` 1.0)
  (bind (_direction _ducky) (`Timeline|Timeline` :!via `PlayFromStart`)
    (:`Update`
      ; Gets the first item of the array and flips that item back down
      (`SceneComponent.K2_SetRelativeRotation` _output (`KismetMathLibrary.RLerp` (`SceneComponent.RelativeRotation` _output) (struct :`Roll` -90.0) _ducky) false false))
    (:`Finished`
      ; QUEUE:  leaves item 0, then shifts each item one down ( 1 -> 0 , 2 -> 1 ETC ), loops until every item in the array is pushed down one
      (`KismetArrayLibrary.Array_Remove` _queue)
      (for (_array_element _array_index) _queue
        (if (not (== _array_index 0))
          (bind _returnvalue (`KismetArrayLibrary.Array_Add` _queue _array_element))
          (`KismetArrayLibrary.Array_Remove` _queue (- _returnvalue 1)))))))

(fn `UserConstructionScript`)