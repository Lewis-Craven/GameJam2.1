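; BP_ShootingDuck1 is a shooting-gallery target duck that repeatedly pops up and drops back down.
; A random-delay loop plays a timeline rotating the duck up, then a second timeline lowers it after it lingers, tracked by IsUp.
; Interact while up adds to the first-person character's Score and reuses the lowering timeline.
; Interact also swaps the duck to a spook material once Score reaches a threshold.
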(event `ReLoop`
  (bind _duck (`self.Duck`))
  (`GameplayStatics.GetActorOfClass` "/Game/FirstPerson/Blueprints/BP_FirstPersonCharacter.BP_FirstPersonCharacter_C" :!label _label)
  (`KismetSystemLibrary.Delay` (`KismetMathLibrary.RandomFloatInRange` 0.8 4.5))
  (if (`self.IsUp?`)
    (`self.ReLoop`)
    (else
      (bind (_direction _newtrack_0) (`Timeline|Timeline` :!via `PlayFromStart`)
        (:`Update`
          (`SceneComponent.K2_SetRelativeRotation` _duck (`KismetMathLibrary.RLerp` (`SceneComponent.RelativeRotation` _duck) (struct) _newtrack_0 true) false false))
        (:`Finished`
          (set `self.IsUp?` true)
          (`self.Linger`))))))

(event `self.ReceiveBeginPlay`
  (goto _label))

(event `Linger`
  (`KismetSystemLibrary.Delay` 3.0)
  (if (`self.IsUp?`)
    (bind (_direction _newtrack_0) (`Timeline|Timeline_0` :!via `PlayFromStart` :!label _label_2)
      (:`Update`
        (`SceneComponent.K2_SetRelativeRotation` (`self.Duck`) (`KismetMathLibrary.RLerp` (`SceneComponent.RelativeRotation` (`self.Duck`)) (struct :`Roll` -90.0) _newtrack_0 true) false false))
      (:`Finished`
        (set `self.IsUp?` false)
        (`KismetSystemLibrary.Delay` 0.5)
        (`self.ReLoop`)))))

(event `self.Interact`
  (bind _asbp_first_person_character (cast `/Game/FirstPerson/Blueprints/BP_FirstPersonCharacter` (`GameplayStatics.GetPlayerPawn` 0)))
  (if (>= (`/Game/FirstPerson/Blueprints/BP_FirstPersonCharacter.Score` _asbp_first_person_character) 18)
    (`PrimitiveComponent.SetMaterial` (`self.Duck`) 1 "/Game/Assets/Materials/TargetDuckSpooks.TargetDuckSpooks"))
  (if (`self.IsUp?`)
    (`/Engine/EditorBlueprintResources/StandardMacros.IncrementInt` (`/Game/FirstPerson/Blueprints/BP_FirstPersonCharacter.Score` _asbp_first_person_character)
      (:`  `
        (goto _label_2 :!via `PlayFromStart`)))))

(fn `UserConstructionScript`)