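; BP_LevelLoader is an interactable that sends the player from the horror game into one of four minigame levels: shooter, Simon Says, maze or red light/green light.
; On Interact it calls HorrorSave on the first-person character, then maps its Selection to an index in GI_HorrorSaver's GamesDone array.
; If that entry is unset, it marks it done before opening the matching level, so each minigame loads only once.
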(event `/Game/Lewis-Craven/BPI_Interact.Interact`
  (bind _listselector (`self.listSelector`))
  (bind _asgi_horror_saver (cast `/Game/BARTOSZ_BLUEPRINTS/GI_HorrorSaver` (`GameplayStatics.GetGameInstance`)))
  (bind _asbp_first_person_character (cast `/Game/FirstPerson/Blueprints/BP_FirstPersonCharacter` (`GameplayStatics.GetPlayerPawn` 0)))
  (`/Game/FirstPerson/Blueprints/BP_FirstPersonCharacter.HorrorSave` _asbp_first_person_character)
  (switch `/Game/BARTOSZ_BLUEPRINTS/Enum_LevelSelector` (`self.Selection`)
    (:`NewEnumerator0`
      (set `self.listSelector` 0))
    (:`NewEnumerator1`
      (set `self.listSelector` 1))
    (:`NewEnumerator2`
      (set `self.listSelector` 2))
    (:`NewEnumerator3`
      (set `self.listSelector` 3)))
  (bind _gamesdone (`/Game/BARTOSZ_BLUEPRINTS/GI_HorrorSaver.GamesDone` _asgi_horror_saver))
  (if (not (`|GetArrayItem` _gamesdone _listselector))
    (`KismetArrayLibrary.Array_Set` _gamesdone _listselector true)
    (switch `/Game/BARTOSZ_BLUEPRINTS/Enum_LevelSelector` (`self.Selection`)
      (:`NewEnumerator0`
        (`GameplayStatics.OpenLevelBySoftObjectPtr` "/Game/BARTOSZ_BLUEPRINTS/Shooter_Minigame.Shooter_Minigame"))
      (:`NewEnumerator1`
        (`GameplayStatics.OpenLevelBySoftObjectPtr` "/Game/LucasWan/Map/SimonLvl.SimonLvl"))
      (:`NewEnumerator2`
        (`GameplayStatics.OpenLevelBySoftObjectPtr` "/Game/Cameron/Lanza(Maze)/EvilMazeMap.EvilMazeMap"))
      (:`NewEnumerator3`
        (`GameplayStatics.OpenLevelBySoftObjectPtr` "/Game/Cameron/RedlightGreenlight/RedlightGreenlight.RedlightGreenlight")))))

(fn `UserConstructionScript`)