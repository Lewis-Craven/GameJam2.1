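; BP_Doohicky0 is a Red Light, Green Light controller that alternates between go and stop at random intervals.
; Tick starts an RLGL timer with a random MinDelay–MaxDelay delay whenever none is active.
; RLGL clears ActiveTimer, flips IsGo and prints debug text.
; The BP_Spinner rotation nodes are unconnected, and the printed delay is a separate random roll from the timer's.
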(event `self.ReceiveBeginPlay`)

(event `self.ReceiveTick`
  (params (DeltaSeconds :type "Float (single-precision)"))
  (bind _returnvalue (`KismetMathLibrary.RandomFloatInRange` (`self.MinDelay`) (`self.MaxDelay`)))
  (if (not (`self.ActiveTimer`))
    (set `self.ActiveTimer` true)
    (`KismetSystemLibrary.K2_SetTimer` null "RLGL" _returnvalue false true)
    (`KismetSystemLibrary.PrintString` (`KismetStringLibrary.Conv_DoubleToString` _returnvalue))))

(fn `RLGL`
  (`KismetSystemLibrary.PrintString` "timertime")
  (set `self.ActiveTimer` false)
  (if (`self.IsGo`)
    (set `self.IsGo` false)
    (`KismetSystemLibrary.PrintString` "red")
    (else
      (set `self.IsGo` true)
      (`KismetSystemLibrary.PrintString` "green"))))

(fn `UserConstructionScript`)