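; Red Light Green Light traffic light that sends the player back to their BeginPlay location if caught moving on red.
; A randomly delayed timer flip-flops IsGo and plays a timeline rotating the Spinner, whose updates re-arm the next switch.
; On red, a short grace period precedes per-tick velocity checks, and violations trigger a Fling timeline that lerps the player to the start.
; Disabled older logic and an uncalled RLGL function remain.
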(event `self.ReceiveBeginPlay`
  ; Gets the player starting location and saves it for reset then calls the loop
  (bind _asbp_first_person_character (cast `/Game/FirstPerson/Blueprints/BP_FirstPersonCharacter` (`GameplayStatics.GetPlayerCharacter` 0)))
  (set `self.StartLocation` (`self.K2_GetActorLocation` _asbp_first_person_character))
  (`self.TrafficLightLoop`))

(event `TrafficLightLoop`
  ; Loop begins, creates a timer or random length within set bounds, the timer then calls the colour change Event
  (`KismetSystemLibrary.K2_SetTimerDelegate` (delegate `RedLightGreenLight`) (`KismetMathLibrary.RandomFloatInRange` (`self.MinDelay`) (`self.MaxDelay`))))

(event `RedLightGreenLight`
  (bind _returnvalue (`GameplayStatics.GetPlayerCharacter` 0))
  ; Flip Flops between red and green, the timeline animation plays and then the loop calls itself again. player is allowed to move until red sign is fully raised/ the safty timer ends, once either of these occour the player movement check event is activated
  (`/Engine/EditorBlueprintResources/StandardMacros.FlipFlop`
    (:`A`
      (set `self.IsGo` true)
      (bind (_direction _togreen) (`Timeline|Timeline_2` :!via `Reverse` :!label _label)
        (:`Update`
          (`SceneComponent.K2_SetWorldRotation` (`self.Spinner`) (`KismetMathLibrary.RLerp` (struct :`Roll` 45.0) (struct :`Roll` -45.0) _togreen) false false)
          (if (not (`self.IsGo`))
            (set `self.SafeTime` true)
            (`KismetSystemLibrary.K2_SetTimerDelegate` (delegate `PlayerMoveCheck`) 0.4))
          (`self.TrafficLightLoop`))
        (:`Finished`
          (if (not (`self.IsGo`))
            ; First activation disables the safty timer so player movement can be checked ever frame until the light turns green again, checks player velocity and if they are moving teleports them back to the beginning
            (set `self.SafeTime` false :!label _label_2)
            (if (and (>= (`KismetMathLibrary.VSize` (`MovementComponent.Velocity` (`Character.CharacterMovement` _returnvalue))) 15.0) (not (`self.IsGo`))) :!label _label_3
              (set `self.Flung` true)
              (bind _asbp_first_person_character (cast `/Game/FirstPerson/Blueprints/BP_FirstPersonCharacter` _returnvalue))
              (bind _asbp_first_person_character_2 (cast `/Game/FirstPerson/Blueprints/BP_FirstPersonCharacter` (`GameplayStatics.GetPlayerCharacter` 0)))
              (set `self.CurLoco` (`self.K2_GetActorLocation` _asbp_first_person_character_2))
              (bind (_direction_2 _newtrack_0) (`Timeline|Fling` :!via `PlayFromStart`)
                (:`Update`
                  (`self.K2_SetActorLocation` _asbp_first_person_character (`KismetMathLibrary.VLerp` (`self.CurLoco`) (`self.StartLocation`) _newtrack_0) false false)
                  (`PrimitiveComponent.SetPhysicsLinearVelocity` (`Character.CapsuleComponent` _asbp_first_person_character) (0.0 0.0 0.0) false "None"))
                (:`Finished`
                  (set `self.Flung` false))))))))
    (:`B`
      (set `self.IsGo` false)
      (goto _label))))

(event `self.ReceiveTick`
  (params (DeltaSeconds :type "Float (single-precision)"))
  ; First activation disables the safty timer so player movement can be checked ever frame until the light turns green again, checks player velocity and if they are moving teleports them back to the beginning
  (if (not (or (`self.Flung`) (`self.SafeTime`)))
    (goto _label_3)))

(event `PlayerMoveCheck`
  ; First activation disables the safty timer so player movement can be checked ever frame until the light turns green again, checks player velocity and if they are moving teleports them back to the beginning
  (goto _label_2))

(fn `RLGL`
  (bind _light (`self.Light`))
  ; Disables Active Timer allowing for another to be set, sets the light to the opposite of what it was previously and moves the Spinner static mesh to give visual indication
  (set `self.ActiveTimer` false)
  (if (`self.IsGo`)
    (set `self.IsGo` false)
    (`self.K2_SetActorRotation` _light (`KismetMathLibrary.MakeRotator` -45.0) false)
    (else
      (set `self.IsGo` true)
      (`self.K2_SetActorRotation` _light (`KismetMathLibrary.MakeRotator` 45.0) false))))

(fn `UserConstructionScript`)