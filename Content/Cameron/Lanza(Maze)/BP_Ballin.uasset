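; BP_Ballin is a physics ball actor, in a maze folder, that resets itself when it leaves its allowed height range.
; BeginPlay stores its starting location.
; Each tick it checks its Z against a Resetheight floor and a fixed ceiling, and ResetBall moves it back to the start and zeroes the linear velocity of its Boll component.
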(event `self.ReceiveBeginPlay`
  ; Sets the starting position as a variable so they may be used as reset coordinates
  (set `self.StartCo-ords` (`self.K2_GetActorLocation`)))

(event `self.ReceiveTick`
  (params (DeltaSeconds :type "Float (single-precision)"))
  (bind (_returnvalue_x _returnvalue_y _returnvalue_z) (`KismetMathLibrary.BreakVector` (`self.K2_GetActorLocation`)))
  (bind (_returnvalue_x_2 _returnvalue_y_2 _returnvalue_z_2) (`KismetMathLibrary.BreakVector` (`self.K2_GetActorLocation`)))
  ; Checks every tick if the ball has exceded maximum or minimum height values and resets it if it has
  (if (< _returnvalue_z_2 (`self.resetheight`))
    (`self.ResetBall` :!label _label)
    (elif (> _returnvalue_z 500.0)
      (goto _label))))

(fn `ResetBall`
  ; Teleports the ball to its starting coordinates and removes its velocity
  (`self.K2_SetActorLocation` (`self.StartCo-ords`))
  (`PrimitiveComponent.SetPhysicsLinearVelocity` (`self.Boll`) (0.0 0.0 0.0) false "None"))

(fn `UserConstructionScript`)