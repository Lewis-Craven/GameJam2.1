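; Maze board controller that lets the player tilt the SMBoardtest board through the BoardTiltForward and BoardTiltRight input axes.
; Each axis adds pitch or roll scaled by RotSpeed, then a shared step clamps both within a small symmetric range and pins yaw to zero.
; An older W-key scheme using gates, Tick and a timer flag, apparently to ease pitch back toward level, remains mostly disabled.
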(event `InputAxis|BoardTiltForward`
  (params (AxisValue :type "Float (single-precision)"))
  (bind _sm_boardtest (`self.SM_boardtest`))
  (bind (_returnvalue_roll _returnvalue_pitch _returnvalue_yaw) (`KismetMathLibrary.BreakRotator` (`SceneComponent.K2_GetComponentRotation` _sm_boardtest)))
  ; InputAxis BoardTiltForward
  (`SceneComponent.K2_AddWorldRotation` (`self.SM_boardtest`) (`KismetMathLibrary.MakeRotator` 0.0 (* AxisValue (`self.RotSpeed`))) false false)
  (`SceneComponent.K2_SetWorldRotation` _sm_boardtest (`KismetMathLibrary.MakeRotator` (`KismetMathLibrary.FClamp` _returnvalue_roll -10.0 10.0) (`KismetMathLibrary.FClamp` _returnvalue_pitch -10.0 10.0) (`KismetMathLibrary.FClamp` _returnvalue_yaw 0.0 0.0)) false false :!label _label))

(event `InputAxis|BoardTiltRight`
  (params (AxisValue :type "Float (single-precision)"))
  ; InputAxis BoardTiltRight
  (`SceneComponent.K2_AddWorldRotation` (`self.SM_boardtest`) (`KismetMathLibrary.MakeRotator` (* AxisValue (`self.RotSpeed`))) false false)
  (goto _label))

(fn `UserConstructionScript`)