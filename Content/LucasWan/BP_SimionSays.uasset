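; Simon Says style actor with four directional buttons that visibly press in while the arrow keys are held; it contains no sequence or scoring logic.
; BeginPlay stores each button's start location and a pressed location that changes only its Y.
; Each key plays its own Timeline to lerp a button between the two and reverses it on release.
; Left and Right keys drive the oppositely named components.
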(event `self.ReceiveBeginPlay`
  (`|ExecutionSequence`
    (:`then_0`
      (bind _output_get (set `self.TopStartlocation` (`SceneComponent.RelativeLocation` (`self.top`))))
      (set `self.TopPressedlocation` (`KismetMathLibrary.MakeVector` (.x _output_get) -40.0 (.z _output_get))))
    (:`then_1`
      (bind _output_get_2 (set `self.DownStartlocation` (`SceneComponent.RelativeLocation` (`self.bottom`))))
      (set `self.DownPressedlocation` (`KismetMathLibrary.MakeVector` (.x _output_get_2) -40.0 (.z _output_get_2))))
    (:`then_2`
      (bind _output_get_3 (set `self.LeftStartlocation` (`SceneComponent.RelativeLocation` (`self.left`))))
      (set `self.LeftPressedlocation` (`KismetMathLibrary.MakeVector` (.x _output_get_3) -40.0 (.z _output_get_3))))
    (:`then_3`
      (bind _output_get_4 (set `self.RightStartlocation` (`SceneComponent.RelativeLocation` (`self.right`))))
      (set `self.RightPressedlocation` (`KismetMathLibrary.MakeVector` (.x _output_get_4) -40.0 (.z _output_get_4))))))

(event `Key|Up`
  (params (Key :type "Key Structure"))
  (:`Pressed`
    (bind (_direction _time) (`Timeline|Timeline` :!label _label)
      (:`Update`
        (`SceneComponent.K2_SetRelativeLocation` (`self.top`) (`KismetMathLibrary.VLerp` (`self.TopStartlocation`) (`self.TopPressedlocation`) _time) false false))))
  (:`Released`
    (goto _label :!via `Reverse`)))

(event `Key|Down`
  (params (Key :type "Key Structure"))
  (:`Pressed`
    (bind (_direction _time) (`Timeline|Timeline_0` :!label _label_2)
      (:`Update`
        (`SceneComponent.K2_SetRelativeLocation` (`self.bottom`) (`KismetMathLibrary.VLerp` (`self.DownStartlocation`) (`self.DownPressedlocation`) _time) false false))))
  (:`Released`
    (goto _label_2 :!via `Reverse`)))

(event `Key|Right`
  (params (Key :type "Key Structure"))
  (:`Pressed`
    (bind (_direction _time) (`Timeline|Timeline_1` :!label _label_3)
      (:`Update`
        (`SceneComponent.K2_SetRelativeLocation` (`self.left`) (`KismetMathLibrary.VLerp` (`self.LeftStartlocation`) (`self.LeftPressedlocation`) _time) false false))))
  (:`Released`
    (goto _label_3 :!via `Reverse`)))

(event `Key|Left`
  (params (Key :type "Key Structure"))
  (:`Pressed`
    (bind (_direction _time) (`Timeline|Timeline_2` :!label _label_4)
      (:`Update`
        (`SceneComponent.K2_SetRelativeLocation` (`self.right`) (`KismetMathLibrary.VLerp` (`self.RightStartlocation`) (`self.RightPressedlocation`) _time) false false))))
  (:`Released`
    (goto _label_4 :!via `Reverse`)))

(fn `UserConstructionScript`)