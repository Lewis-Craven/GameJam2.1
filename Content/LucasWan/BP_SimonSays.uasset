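; BP_SimonSays runs a Simon Says minigame with four coloured buttons, locking player movement and look, showing the cursor and moving the first-person camera to its own.
; Mouse clicks trace under the cursor, glow the hit button and pass its colour to RegisterInput; GlowButton lights buttons by Step.
; Round events drive score, sounds and widgets, resetting on failure.
; Winning past the score threshold saves HorrorCounter progress and fades into the circus level.
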(event `self.ReceiveBeginPlay`
  (bind _returnvalue (`GameplayStatics.GetPlayerController` 0))
  (`WidgetBlueprintLibrary.SetInputMode_GameAndUIEx` _returnvalue null)
  (set `PlayerController.bShowMouseCursor` true _returnvalue)
  (bind _returnvalue_2 (`|CreateWidget` "/Game/LucasWan/UI/UI_SimonScore.UI_SimonScore_C"))
  (`UserWidget.AddToViewport` _returnvalue_2 0)
  (bind _asbp_first_person_character (cast `/Game/FirstPerson/Blueprints/BP_FirstPersonCharacter` (`GameplayStatics.GetPlayerPawn` 0)))
  (`SceneComponent.K2_SetWorldLocation` (`/Game/FirstPerson/Blueprints/BP_FirstPersonCharacter.FirstPersonCamera` _asbp_first_person_character) (`SceneComponent.K2_GetComponentLocation` (`self.Camera`)) false false)
  (bind _returnvalue_3 (`PlayerState.GetPlayerController` (`Pawn.PlayerState` _asbp_first_person_character)))
  (set `PlayerController.bShowMouseCursor` true _returnvalue_3)
  (set `/Game/FirstPerson/Blueprints/BP_FirstPersonCharacter.IsInShooterOrMaze` true _asbp_first_person_character)
  (`Controller.SetIgnoreMoveInput` _returnvalue_3 true)
  (`Controller.SetIgnoreLookInput` _returnvalue_3 true)
  (set `Character.JumpMaxCount` 0 _asbp_first_person_character)
  (bind _returnvalue_4 (`|CreateWidget` "/Game/LucasWan/UI/UI_SimonObjective.UI_SimonObjective_C"))
  (`UserWidget.AddToViewport` _returnvalue_4 0)
  (`KismetSystemLibrary.Delay` 2.0)
  (`Widget.RemoveFromParent` _returnvalue_4))

(event `Key|LeftMouseButton`
  (params (Key :type "Key Structure"))
  (bind (_worldlocation _worlddirection) (`PlayerController.DeprojectMousePositionToWorld` (`GameplayStatics.GetPlayerController` 0)))
  (:`Pressed`
    (bind (_outhit _returnvalue) (`KismetSystemLibrary.LineTraceSingle` _worldlocation (+ _worldlocation (* _worlddirection 10000.0)) "TraceTypeQuery1"))
    (if _returnvalue
      (`|ExecutionSequence`
        (:`then_0`
          (bind (_bblockinghit _binitialoverlap _time _distance _location _impactpoint _normal _impactnormal _physmat _hitactor) (`GameplayStatics.BreakHitResult` _outhit))
          (bind _asbp_red_button (cast `/Game/LucasWan/BP_RedButton` _hitactor))
          (`/Game/LucasWan/BP_RedButton.Glow` _asbp_red_button)
          (`self.registerInput` "Red"))
        (:`then_1`
          (bind _asbp_blue_button (cast `/Game/LucasWan/BP_BlueButton` _hitactor))
          (`/Game/LucasWan/BP_BlueButton.Glow` _asbp_blue_button)
          (`self.registerInput` "Blue"))
        (:`then_2`
          (bind _asbp_green_button (cast `/Game/LucasWan/BP_GreenButton` _hitactor))
          (`/Game/LucasWan/BP_GreenButton.Glow` _asbp_green_button)
          (`self.registerInput` "Green"))
        (:`then_3`
          (bind _asbp_yellow_button (cast `/Game/LucasWan/BP_YellowButton` _hitactor))
          (`/Game/LucasWan/BP_YellowButton.Glow` _asbp_yellow_button)
          (`self.registerInput` "Yellow"))))))

(event `self.glowButton`
  (switch `ESimonButtonType` (`self.Step`)
    (:`Red`
      (bind _returnvalue (`GameplayStatics.GetActorOfClass` "/Game/LucasWan/BP_RedButton.BP_RedButton_C"))
      (`/Game/LucasWan/BP_RedButton.Glow` _returnvalue))
    (:`Blue`
      (bind _returnvalue_2 (`GameplayStatics.GetActorOfClass` "/Game/LucasWan/BP_BlueButton.BP_BlueButton_C"))
      (`/Game/LucasWan/BP_BlueButton.Glow` _returnvalue_2))
    (:`Yellow`
      (bind _returnvalue_3 (`GameplayStatics.GetActorOfClass` "/Game/LucasWan/BP_YellowButton.BP_YellowButton_C"))
      (`/Game/LucasWan/BP_YellowButton.Glow` _returnvalue_3))
    (:`Green`
      (bind _returnvalue_4 (`GameplayStatics.GetActorOfClass` "/Game/LucasWan/BP_GreenButton.BP_GreenButton_C"))
      (`/Game/LucasWan/BP_GreenButton.Glow` _returnvalue_4))))

(event `Winner`
  ; Update to return to level
  (bind _asbp_first_person_character (cast `/Game/FirstPerson/Blueprints/BP_FirstPersonCharacter` (`GameplayStatics.GetPlayerPawn` 0)))
  (`/Engine/EditorBlueprintResources/StandardMacros.IncrementFloat` (`/Game/FirstPerson/Blueprints/BP_FirstPersonCharacter.HorrorCounter` _asbp_first_person_character)
    (:`  `
      (`/Game/FirstPerson/Blueprints/BP_FirstPersonCharacter.HorrorSave` _asbp_first_person_character)
      (bind _returnvalue (`|CreateWidget` "/Game/Cameron/RedlightGreenlight/BPW_Black.BPW_Black_C"))
      (`UserWidget.AddToViewport` _returnvalue 0)
      (`/Game/Cameron/RedlightGreenlight/BPW_Black.Fade` _returnvalue)
      (`KismetSystemLibrary.Delay` 1.0)
      (`GameplayStatics.OpenLevelBySoftObjectPtr` "/Game/Ethan/Level/Lvl_Circus.Lvl_Circus"))))

(event `self.ReceiveTick`
  (params (DeltaSeconds :type "Float (single-precision)")))

(event `self.onRoundWon`
  (if (>= (`self.SimonScore`) 4)
    (`self.Winner`)
    (else
      (`GameplayStatics.PlaySound2D` "/Game/LucasWan/Sound/SW_Winner.SW_Winner" 1.0 1.0 0.0 null null)
      (bind _returnvalue (`|CreateWidget` "/Game/LucasWan/UI/UI_WOO.UI_WOO_C"))
      (`UserWidget.AddToViewport` _returnvalue 0)
      (`KismetSystemLibrary.Delay` 0.4)
      (`Widget.RemoveFromParent` _returnvalue)
      (`/Engine/EditorBlueprintResources/StandardMacros.IncrementInt` (`self.SimonScore`)))))

(event `self.onGameOver`
  (set `self.FinalSimonScore` (`self.SimonScore`))
  (bind _returnvalue (`|CreateWidget` "/Game/LucasWan/UI/UI_BOO.UI_BOO_C"))
  (`UserWidget.AddToViewport` _returnvalue 0)
  (`GameplayStatics.PlaySound2D` "/Game/LucasWan/Sound/SW_GameOver.SW_GameOver" 1.0 1.0 0.0 null null)
  (`KismetSystemLibrary.Delay` 1.0)
  (`self.resetGame`)
  (`Widget.RemoveFromParent` _returnvalue)
  (set `self.SimonScore` 0)
  (set `self.FinalSimonScore` 0))

(event `self.mouseCursor`
  (bind _returnvalue (`GameplayStatics.GetActorOfClass` "/Game/FirstPerson/Blueprints/BP_FirstPersonPlayerController.BP_FirstPersonPlayerController_C"))
  (`/Engine/EditorBlueprintResources/StandardMacros.FlipFlop`
    (:`A`
      (set `PlayerController.bShowMouseCursor` false _returnvalue))
    (:`B`
      (set `PlayerController.bShowMouseCursor` true _returnvalue))))

(fn `UserConstructionScript`)