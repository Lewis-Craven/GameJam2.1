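; BP_TentDoor is a tent door that lifts when a player with a high enough HorrorCounter enters its trigger box, and returns the player to the starter level after they leave.
; A Timeline lerps the mesh upward on overlap and reverses on exit.
; Exit also arms LevelTransition, so when the Timeline finishes, it resets the GI_HorrorSaver counter and opens Lvl_StarterLevel after a short delay.
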(event `self.Box.OnComponentBeginOverlap`
  (params (OverlappedComponent :type "PrimitiveComponent Object Reference") (OtherActor :type "Actor Object Reference") (OtherComp :type "PrimitiveComponent Object Reference") (OtherBodyIndex :type Integer) (bFromSweep :type Boolean) (SweepResult :type "HitResult Structure (by ref)"))
  (bind _scale (`self.Scale`))
  (bind _rotation (`self.Rotation`))
  (bind _asbp_first_person_character (cast `/Game/FirstPerson/Blueprints/BP_FirstPersonCharacter` OtherActor))
  (if (>= (`/Game/FirstPerson/Blueprints/BP_FirstPersonCharacter.HorrorCounter` _asbp_first_person_character) 4.0)
    (bind (_direction _newtrack_0) (`Timeline|Timeline` :!via `PlayFromStart` :!label _label)
      (:`Update`
        (`SceneComponent.K2_SetRelativeTransform` (`self.StaticMesh`) (`KismetMathLibrary.TLerp` (`KismetMathLibrary.MakeTransform` (10.0 -230.0 0.0) _rotation _scale) (`KismetMathLibrary.MakeTransform` (10.0 -230.0 1000.0) _rotation _scale) _newtrack_0) false false))
      (:`Finished`
        (if (`self.LevelTransition`)
          (bind _asgi_horror_saver (cast `/Game/BARTOSZ_BLUEPRINTS/GI_HorrorSaver` (`GameplayStatics.GetGameInstance`)))
          (set `/Game/BARTOSZ_BLUEPRINTS/GI_HorrorSaver.HorrorStorer` 0.0 _asgi_horror_saver)
          (`KismetSystemLibrary.Delay` 0.3)
          (`GameplayStatics.OpenLevelBySoftObjectPtr` "/Game/Lewis-Craven/Lvl_StarterLevel.Lvl_StarterLevel"))))))

(event `self.Box.OnComponentEndOverlap`
  (params (OverlappedComponent :type "PrimitiveComponent Object Reference") (OtherActor :type "Actor Object Reference") (OtherComp :type "PrimitiveComponent Object Reference") (OtherBodyIndex :type Integer))
  (set `self.LevelTransition` true)
  (cast `/Game/FirstPerson/Blueprints/BP_FirstPersonCharacter` OtherActor)
  (if (>= (`/Game/FirstPerson/Blueprints/BP_FirstPersonCharacter.HorrorCounter` (stale `self.Box.OnComponentBeginOverlap` _asbp_first_person_character)) 4.0)
    (goto _label :!via `ReverseFromEnd`)))

(fn `UserConstructionScript`)